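; Player controller for a touch-driven match puzzle that selects a tapped BP_Tile and swipes it to swap with a grid neighbour.
; Touch start and move positions give the swipe direction; Swiping functions swap tiles in the generator's Tiles array and TileLoc map, using ±1 or ±7 index offsets.
; BP_Generator.CheckSwap runs after each direction, and the matching Check function undoes the swap unless Match is set.
; Debug PrintStrings trace clicks and swaps.
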(event Input|EnhancedActionEvents|EnhancedInputActionIA_Click
  (params (ActionValue :type Boolean) (ElapsedSeconds :type Float%20%28double-precision%29) (TriggeredSeconds :type Float%20%28double-precision%29) (InputAction :type Input%20Action%20Object%20Reference :default "/Game/Inputs/IA_Click.IA_Click"))
  (bind (_sucess _clickactor) (CallFunction|GetClickedActor))
  (Development|PrintString (Utilities|GetDisplayName _clickactor) _sucess))

(event EventBeginPlay
  (CallFunction|SetupInput))

(event EventTick
  (params (DeltaSeconds :type Float%20%28single-precision%29)))

(event Input|TouchEvents|Touch1
  (params (Key :type Key%20Structure :default "None"))
  (:Pressed
    (Utilities|FlowControl|DoOnce false :!label _label
      (:Completed
        (bind _asbp_tile (Utilities|Casting|CastToBP_Tile (.ClickActor (CallFunction|GetClickedActor))))
        (Development|PrintString (Utilities|GetDisplayName _asbp_tile))
        (Default|Deselecet (Variables|Default|GetMainTile))
        (Variables|Default|SetMainTile _asbp_tile)
        (Default|Select _asbp_tile))))
  (:Released
    (goto _label Reset)))

(event Input|TouchEvents|InputTouch
  (params (Location :type Vector) (FingerIndex :type ETouchIndex%20Enum))
  (bind _returnvalue (Math|Vector2D|MakeVector2D (.x Location) (.y Location)))
  (bind _maintile (Variables|Default|GetMainTile))
  (bind _maintile_2 (Variables|Default|GetMainTile))
  (bind _gen (Variables|/Game/_blueprints/BP_Tile.BP_Tile_C|GetGen _maintile_2))
  (:Pressed
    (Variables|Default|SetStarPos _returnvalue)
    (Variables|Default|SetTouching true))
  (:Released
    (goto _label Reset))
  (:Moved
    (Utilities|FlowControl|Delay 0.1)
    (Variables|Default|SetEndPos _returnvalue)
    (if (Variables|/Game/_blueprints/BP_Tile.BP_Tile_C|GetSelected (Variables|Default|GetMainTile))
      (Utilities|FlowControl|DoOnce false :!label _label
        (:Completed
          (Utilities|FlowControl|Sequence
            (:then_0
              (CallFunction|SwipingLeft _maintile)
              (bind _asbp_generator (Utilities|Casting|CastToBP_Generator _gen))
              (Default|CheckSwap _asbp_generator)
              (CallFunction|CheckLeft _gen))
            (:then_1
              (CallFunction|SwipingRight _maintile)
              (bind _asbp_generator_2 (Utilities|Casting|CastToBP_Generator _gen))
              (Default|CheckSwap _asbp_generator_2)
              (CallFunction|CheckRight _gen))
            (:then_2
              (CallFunction|SwipingUp _maintile_2)
              (bind _asbp_generator_3 (Utilities|Casting|CastToBP_Generator _gen))
              (Default|CheckSwap _asbp_generator_3)
              (CallFunction|CheckUp _gen))
            (:then_3
              (CallFunction|SwipingDown _maintile_2)
              (bind _asbp_generator_4 (Utilities|Casting|CastToBP_Generator _gen))
              (Default|CheckSwap _asbp_generator_4)
              (CallFunction|CheckDown _gen))
            (:then_4
              (Default|Deselecet (Variables|Default|GetMainTile)))))))))

(fn ConstructionScript)

(fn GetClickedActor
  (bind (_hitresult _returnvalue) (Game|Player|GetHitResultUnderCursorbyChannel "TraceTypeQuery1" true))
  (bind _hitactor (Collision|BreakHitResult _hitresult))
  (return (and _returnvalue (Utilities|DoesObjectImplementInterface _hitactor "/Game/_blueprints/BPI_Interactable.BPI_Interactable_C")) _hitactor))

(fn SetupInput
  (bind _returnvalue (PlayerController|LocalPlayerSubsystems|GetEnhancedInputLocalPlayerSubsystem))
  (Utilities|IsValid _returnvalue
    (:Is%20Valid
      (Input|AddMappingContext _returnvalue "/Game/Inputs/IMC_General.IMC_General" 0 "(bIgnoreAllPressedKeysUntilRelease=True,bForceImmediately=False,bNotifyUserSettings=False)"))))

(fn SwipingLeft
  (params (Tile :type BP%20Tile%20Object%20Reference%20%28by%20ref%29))
  (bind _gen (Variables|/Game/_blueprints/BP_Tile.BP_Tile_C|GetGen Tile))
  (bind _tiles (Variables|/Game/_blueprints/BP_Generator.BP_Generator_C|GetTiles _gen))
  (bind _tileloc (Variables|/Game/_blueprints/BP_Generator.BP_Generator_C|GetTileLoc _gen))
  (bind (_value _returnvalue) (Utilities|Map|Find _tileloc Tile))
  (if (Variables|/Game/_blueprints/BP_Tile.BP_Tile_C|GetCanLeft Tile)
    (if (> (.x (- (Variables|Default|GetStarPos) (Variables|Default|GetEndPos))) (Variables|Default|GetDragAmt))
      (if _returnvalue
        (bind _output_get (Variables|Default|SetOrig _value))
        (bind _output_get_2 (Variables|Default|SetOtherTileNum (- _value 1)))
        (Default|SwapRight Tile)
        (Default|SwapLeft (Utilities|Array|Get(acopy) _tiles _output_get_2))
        (Development|PrintString (Utilities|String|Append (Utilities|String|ToString(Integer) _output_get) " AND THE " (Utilities|String|ToString(Integer) _output_get_2)))
        (Utilities|Array|SetArrayElem _tiles (Variables|Default|GetOrig) (Utilities|Array|Get(acopy) _tiles _output_get_2))
        (Utilities|Array|SetArrayElem _tiles (Variables|Default|GetOtherTileNum) Tile)
        (Utilities|Map|Add _tileloc (Utilities|Array|Get(acopy) _tiles _output_get_2) (Variables|Default|GetOrig))
        (Utilities|Map|Add _tileloc Tile (Variables|Default|GetOtherTileNum))
        (Variables|Default|SetOrig (Variables|Default|GetOtherTileNum))
        (Variables|Default|SetOtherTileNum (Variables|Default|GetOrig))
        (Development|PrintString (Utilities|String|Append "FThe value at " (Utilities|String|ToString(Integer) (Variables|Default|GetOrig)) " is:" (Utilities|GetDisplayName (Utilities|Array|Get(acopy) _tiles _output_get_2))))
        (Development|PrintString (Utilities|String|Append "FThe value at " (Utilities|String|ToString(Integer) _output_get_2) " is:" (Utilities|GetDisplayName Tile)))))))

(fn SwipingRight
  (params (Tile :type BP%20Tile%20Object%20Reference))
  (bind _gen (Variables|/Game/_blueprints/BP_Tile.BP_Tile_C|GetGen Tile))
  (bind _tiles (Variables|/Game/_blueprints/BP_Generator.BP_Generator_C|GetTiles _gen))
  (bind _tileloc (Variables|/Game/_blueprints/BP_Generator.BP_Generator_C|GetTileLoc _gen))
  (bind (_value _returnvalue) (Utilities|Map|Find _tileloc Tile))
  (if (Variables|/Game/_blueprints/BP_Tile.BP_Tile_C|GetCanRight Tile)
    ;[0.15 0.15 0.15 0.5] Swipe Right
    (if (< (.x (- (Variables|Default|GetStarPos) (Variables|Default|GetEndPos))) (* (Variables|Default|GetDragAmt) -1.0))
      (if _returnvalue
        (Variables|Default|SetOrig _value)
        (bind _output_get (Variables|Default|SetOtherTileNum (+ _value 1)))
        (Default|SwapLeft Tile)
        (Default|SwapRight (Utilities|Array|Get(acopy) _tiles _output_get))
        (Utilities|Array|SetArrayElem _tiles (Variables|Default|GetOrig) (Utilities|Array|Get(acopy) _tiles _output_get))
        (Utilities|Array|SetArrayElem _tiles (Variables|Default|GetOtherTileNum) Tile)
        (Utilities|Map|Add _tileloc (Utilities|Array|Get(acopy) _tiles _output_get) (Variables|Default|GetOrig))
        (Utilities|Map|Add _tileloc Tile (Variables|Default|GetOtherTileNum))
        (Variables|Default|SetOrig (Variables|Default|GetOtherTileNum))
        (Variables|Default|SetOtherTileNum (Variables|Default|GetOrig))
        (Development|PrintString (Utilities|String|Append "FThe value at " (Utilities|String|ToString(Integer) (Variables|Default|GetOrig)) " is:" (Utilities|GetDisplayName (Utilities|Array|Get(acopy) _tiles _output_get))))
        (Development|PrintString (Utilities|String|Append "FThe value at " (Utilities|String|ToString(Integer) (Variables|Default|GetOtherTileNum)) " is:" (Utilities|GetDisplayName Tile)))))))

(fn SwipingUp
  (params (Tile :type BP%20Tile%20Object%20Reference))
  (bind _gen (Variables|/Game/_blueprints/BP_Tile.BP_Tile_C|GetGen Tile))
  (bind _tiles (Variables|/Game/_blueprints/BP_Generator.BP_Generator_C|GetTiles _gen))
  (bind _tileloc (Variables|/Game/_blueprints/BP_Generator.BP_Generator_C|GetTileLoc _gen))
  (bind (_value _returnvalue) (Utilities|Map|Find _tileloc 0))
  (if (Variables|/Game/_blueprints/BP_Tile.BP_Tile_C|GetCanUp Tile)
    (if (> (.y (- (Variables|Default|GetStarPos) (Variables|Default|GetEndPos))) (Variables|Default|GetDragAmt))
      (if _returnvalue
        (Variables|Default|SetOrig _value)
        (bind _output_get (Variables|Default|SetOtherTileNum (+ _value 7)))
        (Default|SwapDown Tile)
        (Default|SwapUp (Utilities|Array|Get(acopy) _tiles _output_get))
        (Utilities|Array|SetArrayElem _tiles (Variables|Default|GetOrig) (Utilities|Array|Get(acopy) _tiles _output_get))
        (Utilities|Array|SetArrayElem _tiles (Variables|Default|GetOtherTileNum) Tile)
        (Utilities|Map|Add _tileloc (Utilities|Array|Get(acopy) _tiles _output_get) (Variables|Default|GetOrig))
        (Utilities|Map|Add _tileloc Tile (Variables|Default|GetOtherTileNum))
        (Variables|Default|SetOrig (Variables|Default|GetOtherTileNum))
        (Variables|Default|SetOtherTileNum (Variables|Default|GetOrig))
        (Development|PrintString (Utilities|String|Append "FThe value at " (Utilities|String|ToString(Integer) (Variables|Default|GetOrig)) " is:" (Utilities|GetDisplayName (Utilities|Array|Get(acopy) _tiles _output_get))))
        (Development|PrintString (Utilities|String|Append "FThe value at " (Utilities|String|ToString(Integer) _output_get) " is:" (Utilities|GetDisplayName Tile)))))))

(fn SwipingDown
  (params (Tile :type BP%20Tile%20Object%20Reference))
  (bind _gen (Variables|/Game/_blueprints/BP_Tile.BP_Tile_C|GetGen Tile))
  (bind _tiles (Variables|/Game/_blueprints/BP_Generator.BP_Generator_C|GetTiles _gen))
  (bind _tileloc (Variables|/Game/_blueprints/BP_Generator.BP_Generator_C|GetTileLoc _gen))
  (bind (_value _returnvalue) (Utilities|Map|Find _tileloc Tile))
  (if (Variables|/Game/_blueprints/BP_Tile.BP_Tile_C|GetCanDown Tile)
    ;[0.15 0.15 0.15 0.5] Swap Down
    (if (< (.y (- (Variables|Default|GetStarPos) (Variables|Default|GetEndPos))) (* (Variables|Default|GetDragAmt) -1.0))
      (if _returnvalue
        (Variables|Default|SetOrig _value)
        (bind _output_get (Variables|Default|SetOtherTileNum (- _value 7)))
        (Default|SwapUp Tile)
        (Default|SwapDown (Utilities|Array|Get(acopy) _tiles _output_get))
        (Utilities|Array|SetArrayElem _tiles (Variables|Default|GetOrig) (Utilities|Array|Get(acopy) _tiles _output_get))
        (Utilities|Array|SetArrayElem _tiles (Variables|Default|GetOtherTileNum) Tile)
        (Utilities|Map|Add _tileloc (Utilities|Array|Get(acopy) _tiles _output_get) (Variables|Default|GetOrig))
        (Utilities|Map|Add _tileloc Tile (Variables|Default|GetOtherTileNum))
        (Default|CheckSwap _gen)
        (if (Variables|/Game/_blueprints/BP_Generator.BP_Generator_C|GetMatch _gen)
          (Variables|Default|SetOrig (Variables|Default|GetOtherTileNum))
          (Variables|Default|SetOtherTileNum (Variables|Default|GetOrig))
          (Development|PrintString (Utilities|String|Append "FThe value at " (Utilities|String|ToString(Integer) (Variables|Default|GetOrig)) " is:" (Utilities|GetDisplayName (Utilities|Array|Get(acopy) _tiles _output_get))))
          (Development|PrintString (Utilities|String|Append "FThe value at " (Utilities|String|ToString(Integer) (Variables|Default|GetOrig)) " is:" (Utilities|GetDisplayName Tile))))))))

(fn CheckLeft
  (params (Gen :type BP%20Generator%20Object%20Reference))
  (bind _tileloc (Variables|/Game/_blueprints/BP_Generator.BP_Generator_C|GetTileLoc Gen))
  (bind _tiles (Variables|/Game/_blueprints/BP_Generator.BP_Generator_C|GetTiles Gen))
  (if (== (Variables|/Game/_blueprints/BP_Generator.BP_Generator_C|GetMatch Gen) true)
    (Variables|/Game/_blueprints/BP_Generator.BP_Generator_C|SetMatch Gen false)
    (else
      (Default|SwapLeft (.Key (Utilities|Map|GetKeyValueByIndex _tileloc (Variables|Default|GetOrig))))
      (Default|SwapRight (.Key (Utilities|Map|GetKeyValueByIndex _tileloc (Variables|Default|GetOtherTileNum))))
      (Utilities|Array|SetArrayElem _tiles (.Value (Utilities|Map|GetKeyValueByIndex _tileloc (Variables|Default|GetOrig))) (.Key (Utilities|Map|GetKeyValueByIndex _tileloc (Variables|Default|GetOtherTileNum))))
      (Utilities|Array|SetArrayElem _tiles (.Value (Utilities|Map|GetKeyValueByIndex _tileloc (Variables|Default|GetOtherTileNum))) (.Key (Utilities|Map|GetKeyValueByIndex _tileloc (Variables|Default|GetOrig))))
      (Utilities|Map|Add _tileloc (.Key (Utilities|Map|GetKeyValueByIndex _tileloc (Variables|Default|GetOtherTileNum))) (.Value (Utilities|Map|GetKeyValueByIndex _tileloc (Variables|Default|GetOrig))))
      (Utilities|Map|Add _tileloc (.Key (Utilities|Map|GetKeyValueByIndex _tileloc (Variables|Default|GetOrig))) (.Value (Utilities|Map|GetKeyValueByIndex _tileloc (Variables|Default|GetOtherTileNum))))
      (Variables|Default|SetOrig (Variables|Default|GetOtherTileNum))
      (Variables|Default|SetOtherTileNum (Variables|Default|GetOrig))
      (Development|PrintString (Utilities|String|Append "The value at " (Utilities|String|ToString(Integer) (Variables|Default|GetOrig)) " is:" (Utilities|GetDisplayName (.Key (Utilities|Map|GetKeyValueByIndex _tileloc (Variables|Default|GetOrig))))))
      (Development|PrintString (Utilities|String|Append "The value at " (Utilities|String|ToString(Integer) (Variables|Default|GetOtherTileNum)) " is:" (Utilities|GetDisplayName (.Key (Utilities|Map|GetKeyValueByIndex _tileloc (Variables|Default|GetOtherTileNum)))))))))

(fn CheckRight
  (params (Gen :type BP%20Generator%20Object%20Reference))
  (bind _tileloc (Variables|/Game/_blueprints/BP_Generator.BP_Generator_C|GetTileLoc Gen))
  (bind _tiles (Variables|/Game/_blueprints/BP_Generator.BP_Generator_C|GetTiles Gen))
  (if (== (Variables|/Game/_blueprints/BP_Generator.BP_Generator_C|GetMatch Gen) true)
    (Variables|/Game/_blueprints/BP_Generator.BP_Generator_C|SetMatch Gen false)
    (else
      (Default|SwapRight (.Key (Utilities|Map|GetKeyValueByIndex _tileloc (Variables|Default|GetOrig))))
      (Default|SwapLeft (.Key (Utilities|Map|GetKeyValueByIndex _tileloc (Variables|Default|GetOtherTileNum))))
      (Utilities|Array|SetArrayElem _tiles (.Value (Utilities|Map|GetKeyValueByIndex _tileloc (Variables|Default|GetOrig))) (.Key (Utilities|Map|GetKeyValueByIndex _tileloc (Variables|Default|GetOtherTileNum))))
      (Utilities|Array|SetArrayElem _tiles (.Value (Utilities|Map|GetKeyValueByIndex _tileloc (Variables|Default|GetOtherTileNum))) (.Key (Utilities|Map|GetKeyValueByIndex _tileloc (Variables|Default|GetOrig))))
      (Utilities|Map|Add _tileloc (.Key (Utilities|Map|GetKeyValueByIndex _tileloc (Variables|Default|GetOtherTileNum))) (.Value (Utilities|Map|GetKeyValueByIndex _tileloc (Variables|Default|GetOrig))))
      (Utilities|Map|Add _tileloc (.Key (Utilities|Map|GetKeyValueByIndex _tileloc (Variables|Default|GetOrig))) (.Value (Utilities|Map|GetKeyValueByIndex _tileloc (Variables|Default|GetOtherTileNum))))
      (Variables|Default|SetOrig (Variables|Default|GetOtherTileNum))
      (Variables|Default|SetOtherTileNum (Variables|Default|GetOrig))
      (Development|PrintString (Utilities|String|Append "The value at " (Utilities|String|ToString(Integer) (Variables|Default|GetOrig)) " is:" (Utilities|GetDisplayName (.Key (Utilities|Map|GetKeyValueByIndex _tileloc (Variables|Default|GetOrig))))))
      (Development|PrintString (Utilities|String|Append "The value at " (Utilities|String|ToString(Integer) (Variables|Default|GetOtherTileNum)) " is:" (Utilities|GetDisplayName (.Key (Utilities|Map|GetKeyValueByIndex _tileloc (Variables|Default|GetOtherTileNum)))))))))

(fn CheckUp
  (params (Gen :type BP%20Generator%20Object%20Reference))
  (bind _tileloc (Variables|/Game/_blueprints/BP_Generator.BP_Generator_C|GetTileLoc Gen))
  (bind _tiles (Variables|/Game/_blueprints/BP_Generator.BP_Generator_C|GetTiles Gen))
  (if (== (Variables|/Game/_blueprints/BP_Generator.BP_Generator_C|GetMatch Gen) true)
    (Variables|/Game/_blueprints/BP_Generator.BP_Generator_C|SetMatch Gen false)
    (else
      (Default|SwapUp (.Key (Utilities|Map|GetKeyValueByIndex _tileloc (Variables|Default|GetOrig))))
      (Default|SwapDown (.Key (Utilities|Map|GetKeyValueByIndex _tileloc (Variables|Default|GetOtherTileNum))))
      (Utilities|Array|SetArrayElem _tiles (.Value (Utilities|Map|GetKeyValueByIndex _tileloc (Variables|Default|GetOrig))) (.Key (Utilities|Map|GetKeyValueByIndex _tileloc (Variables|Default|GetOtherTileNum))))
      (Utilities|Array|SetArrayElem _tiles (.Value (Utilities|Map|GetKeyValueByIndex _tileloc (Variables|Default|GetOtherTileNum))) (.Key (Utilities|Map|GetKeyValueByIndex _tileloc (Variables|Default|GetOrig))))
      (Utilities|Map|Add _tileloc (.Key (Utilities|Map|GetKeyValueByIndex _tileloc (Variables|Default|GetOtherTileNum))) (.Value (Utilities|Map|GetKeyValueByIndex _tileloc (Variables|Default|GetOrig))))
      (Utilities|Map|Add _tileloc (.Key (Utilities|Map|GetKeyValueByIndex _tileloc (Variables|Default|GetOrig))) (.Value (Utilities|Map|GetKeyValueByIndex _tileloc (Variables|Default|GetOtherTileNum))))
      (Variables|Default|SetOrig (Variables|Default|GetOtherTileNum))
      (Variables|Default|SetOtherTileNum (Variables|Default|GetOrig))
      (Development|PrintString (Utilities|String|Append "The value at " (Utilities|String|ToString(Integer) (.Value (Utilities|Map|GetKeyValueByIndex _tileloc (Variables|Default|GetOrig)))) " is:" (Utilities|GetDisplayName (.Key (Utilities|Map|GetKeyValueByIndex _tileloc (Variables|Default|GetOrig))))))
      (Development|PrintString (Utilities|String|Append "The value at " (Utilities|String|ToString(Integer) (Variables|Default|GetOtherTileNum)) " is:" (Utilities|GetDisplayName (.Key (Utilities|Map|GetKeyValueByIndex _tileloc (Variables|Default|GetOtherTileNum)))))))))

(fn CheckDown
  (params (Gen :type BP%20Generator%20Object%20Reference))
  (bind _tileloc (Variables|/Game/_blueprints/BP_Generator.BP_Generator_C|GetTileLoc Gen))
  (bind _tiles (Variables|/Game/_blueprints/BP_Generator.BP_Generator_C|GetTiles Gen))
  (if (== (Variables|/Game/_blueprints/BP_Generator.BP_Generator_C|GetMatch Gen) true)
    (Variables|/Game/_blueprints/BP_Generator.BP_Generator_C|SetMatch Gen false)
    (else
      (Default|SwapDown (.Key (Utilities|Map|GetKeyValueByIndex _tileloc (Variables|Default|GetOrig))))
      (Default|SwapUp (.Key (Utilities|Map|GetKeyValueByIndex _tileloc (Variables|Default|GetOtherTileNum))))
      (Utilities|Array|SetArrayElem _tiles (.Value (Utilities|Map|GetKeyValueByIndex _tileloc (Variables|Default|GetOrig))) (.Key (Utilities|Map|GetKeyValueByIndex _tileloc (Variables|Default|GetOtherTileNum))))
      (Utilities|Array|SetArrayElem _tiles (.Value (Utilities|Map|GetKeyValueByIndex _tileloc (Variables|Default|GetOtherTileNum))) (.Key (Utilities|Map|GetKeyValueByIndex _tileloc (Variables|Default|GetOrig))))
      (Utilities|Map|Add _tileloc (.Key (Utilities|Map|GetKeyValueByIndex _tileloc (Variables|Default|GetOtherTileNum))) (.Value (Utilities|Map|GetKeyValueByIndex _tileloc (Variables|Default|GetOrig))))
      (Utilities|Map|Add _tileloc (.Key (Utilities|Map|GetKeyValueByIndex _tileloc (Variables|Default|GetOrig))) (.Value (Utilities|Map|GetKeyValueByIndex _tileloc (Variables|Default|GetOtherTileNum))))
      (Variables|Default|SetOrig (Variables|Default|GetOtherTileNum))
      (Variables|Default|SetOtherTileNum (Variables|Default|GetOrig))
      (Development|PrintString (Utilities|String|Append "The value at " (Utilities|String|ToString(Integer) (Variables|Default|GetOrig)) " is:" (Utilities|GetDisplayName (.Key (Utilities|Map|GetKeyValueByIndex _tileloc (Variables|Default|GetOrig))))))
      (Development|PrintString (Utilities|String|Append "The value at " (Utilities|String|ToString(Integer) (Variables|Default|GetOtherTileNum)) " is:" (Utilities|GetDisplayName (.Key (Utilities|Map|GetKeyValueByIndex _tileloc (Variables|Default|GetOtherTileNum)))))))))