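; BP_Tile is a grid tile that takes a random tool type (gear, hammer, lug, plug, screwdriver or wrench) on BeginPlay and sets the matching box material.
; Initialize attaches it to its owner and positions it from GridX/GridY and box bounds.
; NewFunction sets a dynamic material's color for selection, though both colors are black.
; On Destroyed, it writes an incremented DestroyedCount to BP_PlayerController after a one-second delay.
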(event EventBeginPlay
  (bind _box (Variables|Default|GetBox))
  (bind _output_get (Variables|Default|SetColor (.OutItem (Utilities|Array|Random (Utilities|Array|MakeArray "NewEnumerator0" "NewEnumerator1" "NewEnumerator2" "NewEnumerator3" "NewEnumerator4" "NewEnumerator5")))))
  (switch Utilities|FlowControl|Switch|SwitchonColorType _output_get
    (:NewEnumerator0
      (Rendering|Material|SetMaterial _box 0 "/Game/_materials/Block_Textures/M_GearBlock.M_GearBlock"))
    (:NewEnumerator1
      (Rendering|Material|SetMaterial _box 0 "/Game/_materials/Block_Textures/M_Hammer_Block.M_Hammer_Block"))
    (:NewEnumerator2
      (Rendering|Material|SetMaterial _box 0 "/Game/_materials/Block_Textures/M_LW_Block.M_LW_Block"))
    (:NewEnumerator3
      (Rendering|Material|SetMaterial _box 0 "/Game/_materials/Block_Textures/M_Plug_Block.M_Plug_Block"))
    (:NewEnumerator4
      (Rendering|Material|SetMaterial _box 0 "/Game/_materials/Block_Textures/M_SD_Block.M_SD_Block"))
    (:NewEnumerator5
      (Rendering|Material|SetMaterial _box 0 "/Game/_materials/Block_Textures/M_Wrench_Block.M_Wrench_Block"))))

(event EventDestroyed
  (bind _asbp_player_controller (Utilities|Casting|CastToBP_PlayerController (Game|GetPlayerController 0)))
  (Development|PrintString (Utilities|String|ToString(Integer) (Variables|Default|GetDestroyed%20Count)) true true "(R=1.000000,G=0.000000,B=0.013213,A=1.000000)")
  (Utilities|FlowControl|Delay 1.0)
  (bind _output_get (Variables|/Game/_blueprints/BP_PlayerController.BP_PlayerController_C|SetDestroyedCount _asbp_player_controller (+ (Variables|Default|GetDestroyed%20Count) 1)))
  (Development|PrintString (Utilities|String|ToString(Integer) _output_get) true true "(R=1.000000,G=0.000000,B=0.013213,A=1.000000)"))

(fn ConstructionScript)

(fn Initialize
  (bind _returnvalue (Components|GetOwner))
  (Utilities|IsValid _returnvalue
    (:Is%20Valid
      (Transformation|AttachActorToActor _returnvalue "None" "SnapToTarget" "SnapToTarget" "KeepRelative" false)
      (bind _outlocation (CallFunction|CalculateLocation))
      (Transformation|SetActorRelativeLocation _outlocation))))

(fn CalculateLocation
  (bind _box (Variables|Default|GetBox))
  (bind _boxextent (Collision|GetComponentBounds _box))
  (bind (_x _y _z) (Math|Vector|BreakVector _boxextent))
  (return (Math|Vector|MakeVector (* _z (Variables|Default|GetGridX) 2.0) (* _y (Variables|Default|GetGridY) 2.0) 0.0)))

(fn NewFunction
  (params (InSelect :type Boolean))
  (bind _mid (Variables|Material|GetMID)
    (:then
      (Rendering|Material|SetVectorParameterValue _mid "Color" (Math|Color|SelectColor :bPickA InSelect) :!class /Script/Engine.MaterialInstanceDynamic)
      (Development|PrintString (Utilities|GetDisplayName self)))
    (:else
      (return false))))