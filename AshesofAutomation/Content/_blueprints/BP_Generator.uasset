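; BP_Generator runs a match-three board, spawning a 7x7 grid of BP_Tile actors at BeginPlay into a flat array indexed by division and modulo.
; SwapTiles exchanges neighbors, then CheckSwap scans for runs of three or more, destroys them and calls DamageEnemy on GM_Gamemode, or the swap reverts.
; PowerUps clears a row or column by tile type.
; Tile dropping and refilling are unfinished, with empty stubs and debug prints.
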(event EventBeginPlay
  (CallFunction|ClearTiles)
  (CallFunction|IntintializeTiles))

(event Collision|EventActorBeginOverlap
  (params (OtherActor :type Actor%20Object%20Reference)))

(event EventTick
  (params (DeltaSeconds :type Float%20%28single-precision%29)))

(fn ConstructionScript)

(fn IntintializeTiles
  (bind _self self)
  (CallFunction|ClearTiles)
  (for _index (range 0 (- 7 1))
    (for _index_2 (range 0 (- 7 1))
      (bind _returnvalue (Game|SpawnActorfromClass "/Game/_blueprints/BP_Tile.BP_Tile_C" (Math|Transform|MakeTransform (Transformation|GetActorLocation) (Transformation|GetActorRotation)) "AlwaysSpawn" "MultiplyWithRoot" _self _index _index_2 _self 0))
      (Default|Initialize _returnvalue)
      (Utilities|Array|Add (Variables|Default|GetBoard) _returnvalue))))

(fn ClearTiles
  (bind _board (Variables|Default|GetBoard))
  (if (> (Utilities|Array|Length (Variables|Default|GetBoard)) 0)
    (bind _arrayelement (Utilities|Array|ReverseforEachLoop _board)
      (:LoopBody
        (Actor|DestroyActor _arrayelement))
      (:Completed
        (Utilities|Array|Clear _board)))))

(fn SwapTiles
  (params (MainTile :type BP%20Tile%20Object%20Reference) (Dir :type Integer))
  (bind _board (Variables|Default|GetBoard))
  (bind _staticmesh (Variables|/Game/_blueprints/BP_Tile.BP_Tile_C|GetStaticMesh MainTile))
  (Variables|Default|SetNoMatch false)
  (bind _output_get (Variables|Default|SetMainTile MainTile))
  (Variables|Default|SetMain (Utilities|Array|FindItem (Variables|Default|GetBoard) _output_get))
  (Variables|Default|SetMainLoc (Transformation|GetWorldLocation _staticmesh))
  (Utilities|FlowControl|Sequence
    (:then_0
      ;[0.15 0.15 0.15 0.5] Checks Direction of Other Tile
      (if (and (== Dir 1) (!= (Math|Integer|%(Integer) (Utilities|Array|FindItem (Variables|Default|GetBoard) (Variables|Default|GetMainTile)) 7) 0))
        (Variables|Default|SetOther (- (Variables|Default|GetMain) 1))
        (Variables|Default|SetSWAP true :!label _label)))
    (:then_1
      (if (and (== Dir 2) (!= (Math|Integer|%(Integer) (Utilities|Array|FindItem (Variables|Default|GetBoard) (Variables|Default|GetMainTile)) 7) 6))
        (Variables|Default|SetOther (+ (Variables|Default|GetMain) 1))
        (goto _label)))
    (:then_2
      (if (and (== Dir 3) (!= (/ (Utilities|Array|FindItem (Variables|Default|GetBoard) (Variables|Default|GetMainTile)) 7) 6))
        (Variables|Default|SetOther (+ (Variables|Default|GetMain) 7))
        (goto _label)))
    (:then_3
      (if (and (== Dir 4) (!= (/ (Utilities|Array|FindItem (Variables|Default|GetBoard) (Variables|Default|GetMainTile)) 7) 0))
        (Variables|Default|SetOther (- (Variables|Default|GetMain) 7))
        (goto _label)))
    (:then_4
      (Utilities|IsValid (Utilities|Array|Get(acopy) _board (Variables|Default|GetOther))
        (:Is%20Valid
          (Variables|Default|SetOtherTile (Utilities|Array|Get(acopy) _board (Variables|Default|GetOther)))
          (Variables|Default|SetOtherLoc (Transformation|GetWorldLocation (Variables|/Game/_blueprints/BP_Tile.BP_Tile_C|GetStaticMesh (Utilities|Array|Get(acopy) _board (Variables|Default|GetOther)))))
          (Utilities|FlowControl|Sequence
            (:then_0
              (if (Variables|Default|GetSWAP)
                (Transformation|SetWorldLocation _staticmesh (Variables|Default|GetOtherLoc) false false)
                (Transformation|SetWorldLocation (Variables|/Game/_blueprints/BP_Tile.BP_Tile_C|GetStaticMesh (Utilities|Array|Get(acopy) _board (Variables|Default|GetOther))) (Variables|Default|GetMainLoc) false false)
                (Utilities|Array|Swap _board (Variables|Default|GetMain) (Variables|Default|GetOther))
                (Variables|Default|SetSWAP false)))
            (:then_1
              (CallFunction|CheckSwap))
            (:then_2
              (if (Variables|Default|GetNoMatch)
                (Transformation|SetWorldLocation (Variables|/Game/_blueprints/BP_Tile.BP_Tile_C|GetStaticMesh (Variables|Default|GetOtherTile)) (Variables|Default|GetOtherLoc) false false)
                (Transformation|SetWorldLocation (Variables|/Game/_blueprints/BP_Tile.BP_Tile_C|GetStaticMesh (Variables|Default|GetMainTile)) (Variables|Default|GetMainLoc) false false)
                (Utilities|Array|Swap (Variables|Default|GetBoard) (Variables|Default|GetMain) (Variables|Default|GetOther))))
            (:then_3
              (CallFunction|CheckTile))))))))

(fn GetMatchesat
  (params (Index :type Integer))
  (bind _horizontalmatch (LocalVariables|GetHorizontalMatch))
  (bind _verticalmatch (LocalVariables|GetVerticalMatch))
  (bind _horizontalmatch_2 (LocalVariables|GetHorizontalMatch))
  (bind _verticalmatch_2 (LocalVariables|GetVerticalMatch))
  (bind _matchedtiles (Variables|Default|GetMatchedTiles))
  (bind _board (Variables|Default|GetBoard))
  (bind _board_2 (Variables|Default|GetBoard))
  (bind _output (Utilities|Array|Get(acopy) _board_2 Index))
  (LocalVariables|SetColumn (Math|Integer|%(Integer) Index 7))
  (LocalVariables|SetRow (/ Index 7))
  (Utilities|IsValid _output
    (:Is%20Valid
      (LocalVariables|SetCenterTileColor (Variables|/Game/_blueprints/BP_Tile.BP_Tile_C|GetColor _output))
      (Utilities|FlowControl|Sequence
        (:then_0
          ;[0.15 0.15 0.15 0.5] Left
          (bind _output_get (LocalVariables|SetTemp (- Index 1)))
          (Utilities|Array|Clear _horizontalmatch)
          (Utilities|Array|Add _horizontalmatch Index)
          (Utilities|FlowControl|ForLoopwithBreak 0 6 :!label _label
            (:LoopBody
              (if (and (Utilities|Array|IsValidIndex _board_2 _output_get) (Utilities|IsValid (Utilities|Array|Get(acopy) _board_2 _output_get)))
                (if (Math|Boolean|ANDBoolean (>= _output_get 0) (Utilities|Enum|Equal(Enum) (Variables|/Game/_blueprints/BP_Tile.BP_Tile_C|GetColor (Utilities|Array|Get(acopy) _board_2 _output_get)) (LocalVariables|GetCenterTileColor)) (== (/ _output_get 7) (LocalVariables|GetRow)))
                  (Utilities|Array|Add (LocalVariables|GetHorizontalMatch) _output_get)
                  (Math|Integer|DecrementInt _output_get)
                  (else
                    (goto _label Break)))))))
        (:then_1
          ;[0.15 0.15 0.15 0.5] Right
          (bind _output_get_2 (LocalVariables|SetTemp (+ Index 1)))
          (Utilities|FlowControl|ForLoopwithBreak 0 6 :!label _label_2
            (:LoopBody
              (if (Utilities|Array|IsValidIndex _board_2 _output_get_2)
                (if (Math|Boolean|ANDBoolean (< _output_get_2 49) (Utilities|Enum|Equal(Enum) (Variables|/Game/_blueprints/BP_Tile.BP_Tile_C|GetColor (Utilities|Array|Get(acopy) _board_2 _output_get_2)) (LocalVariables|GetCenterTileColor)) (== (/ _output_get_2 7) (LocalVariables|GetRow)))
                  (Utilities|Array|Add (LocalVariables|GetHorizontalMatch) _output_get_2)
                  (Math|Integer|IncrementInt _output_get_2)
                  (else
                    (goto _label_2 Break)))
                (else
                  (goto _label_2 Break))))))
        (:then_2
          (if (< (Utilities|Array|Length _horizontalmatch_2) 3)
            (Utilities|Array|Clear _horizontalmatch_2)))
        (:then_3
          ;[0.15 0.15 0.15 0.5] Down
          (bind _output_get_3 (LocalVariables|SetTemp (- Index 7)))
          (Utilities|Array|Clear _verticalmatch)
          (Utilities|Array|Add _verticalmatch Index)
          (Utilities|FlowControl|ForLoopwithBreak 0 6 :!label _label_3
            (:LoopBody
              (if (Utilities|Array|IsValidIndex _board _output_get_3)
                (if (and (>= _output_get_3 0) (Utilities|Enum|Equal(Enum) (Variables|/Game/_blueprints/BP_Tile.BP_Tile_C|GetColor (Utilities|Array|Get(acopy) _board _output_get_3)) (LocalVariables|GetCenterTileColor)))
                  (Utilities|Array|Add (LocalVariables|GetVerticalMatch) _output_get_3)
                  (LocalVariables|SetTemp (- _output_get_3 7))
                  (else
                    (goto _label_3 Break)))
                (else
                  (goto _label_3 Break))))))
        (:then_4
          ;[0.15 0.15 0.15 0.5] Up
          (bind _output_get_4 (LocalVariables|SetTemp (+ Index 7)))
          (Utilities|FlowControl|ForLoopwithBreak 0 6 :!label _label_4
            (:LoopBody
              (if (Utilities|Array|IsValidIndex _board _output_get_4)
                (if (and (< _output_get_4 49) (Utilities|Enum|Equal(Enum) (Variables|/Game/_blueprints/BP_Tile.BP_Tile_C|GetColor (Utilities|Array|Get(acopy) _board _output_get_4)) (LocalVariables|GetCenterTileColor)))
                  (Utilities|Array|Add (LocalVariables|GetVerticalMatch) _output_get_4)
                  (LocalVariables|SetTemp (+ _output_get_4 7))
                  (else
                    (goto _label_4 Break)))
                (else
                  (goto _label_4 Break))))))
        (:then_5
          (if (< (Utilities|Array|Length _verticalmatch_2) 3)
            (Utilities|Array|Clear _verticalmatch_2)))
        (:then_6
          (for _array_element (LocalVariables|GetHorizontalMatch)
            (Utilities|Array|AddUnique (Variables|Default|GetMatchedTiles) _array_element))
          (for _array_element_2 (LocalVariables|GetVerticalMatch)
            (Utilities|Array|AddUnique _matchedtiles _array_element_2))
          (return _matchedtiles))))
    (:Is%20Not%20Valid
      (return 0))))

(fn ResolveMatches)

(fn FillGrid)

(fn CheckSwap
  (bind _tilestodestory (Variables|Default|GetTilesToDestory))
  (bind _board (Variables|Default|GetBoard))
  (for (_ _array_index) (Variables|Default|GetBoard)
    (bind _matchedtiles (CallFunction|GetMatchesat _array_index))
    (for _array_element _matchedtiles
      (Utilities|Array|AddUnique (Variables|Default|GetTilesToDestory) _array_element)))
  (if true
    (for _array_element_2 _tilestodestory
      (if (Utilities|Array|IsValidIndex _board _array_element_2)
        (Actor|DestroyActor (Utilities|Array|Get(acopy) _board _array_element_2))
        (Utilities|Array|SetArrayElem _board _array_element_2 0)))
    (if (== (Utilities|Array|Length _tilestodestory) 0)
      (Variables|Default|SetNoMatch true)
      (else
        (Utilities|Array|Clear _tilestodestory)
        (bind _asgm_gamemode (Utilities|Casting|CastToGM_Gamemode (Game|GetGameMode)))
        (Utilities|DamageEnemy _asgm_gamemode 1.0)
        (Development|PrintString "Dmg")))))

(fn Deselect
  (for _array_element (Variables|Default|GetBoard)
    (Utilities|IsValid _array_element
      (:Is%20Valid
        (if (Variables|/Game/_blueprints/BP_Tile.BP_Tile_C|GetSelected _array_element)
          (Variables|/Game/_blueprints/BP_Tile.BP_Tile_C|SetSelected _array_element false)
          (Rendering|Material|SetMaterial (Variables|/Game/_blueprints/BP_Tile.BP_Tile_C|GetBox _array_element) 0 (Variables|/Game/_blueprints/BP_Tile.BP_Tile_C|GetOrigMaterial _array_element)))))))

(fn PowerUps
  (params (Tile :type BP%20Tile%20Object%20Reference))
  (bind _board (Variables|Default|GetBoard))
  (bind _board_2 (Variables|Default|GetBoard))
  (bind _color (Variables|/Game/_blueprints/BP_Tile.BP_Tile_C|GetColor Tile))
  (bind _linetodestroy (LocalVariables|GetLineToDestroy))
  (bind _returnvalue (Utilities|Array|FindItem _board_2 Tile))
  (Utilities|FlowControl|Sequence
    (:then_0
      (Utilities|IsValid Tile
        (:Is%20Valid
          (if (Utilities|Enum|Equal(Enum) _color "NewEnumerator6")
            (for (_array_element _array_index) _board
              (if (Math|Boolean|ANDBoolean (== (/ _returnvalue 7) (/ _array_index 7)) (Utilities|Array|IsValidIndex _board _array_index) (Utilities|IsValid _array_element))
                (Utilities|Array|AddUnique _linetodestroy _array_index)))
            (for _array_element_2 _linetodestroy
              (Actor|DestroyActor (Utilities|Array|Get(acopy) (Variables|Default|GetBoard) _array_element_2)))
            (Utilities|Array|Clear _linetodestroy)))))
    (:then_1
      (Utilities|IsValid Tile
        (:Is%20Valid
          (if (Utilities|Enum|Equal(Enum) _color "NewEnumerator7")
            (for (_array_element_3 _array_index_2) _board
              (if (Math|Boolean|ANDBoolean (== (Math|Integer|%(Integer) _returnvalue 7) (Math|Integer|%(Integer) _array_index_2 7)) (Utilities|Array|IsValidIndex _board _array_index_2) (Utilities|IsValid _array_element_3))
                (Utilities|Array|AddUnique _linetodestroy _array_index_2)))
            (for _array_element_4 _linetodestroy
              (Actor|DestroyActor (Utilities|Array|Get(acopy) (Variables|Default|GetBoard) _array_element_4)))
            (Utilities|Array|Clear _linetodestroy)))))
    (:then_2
      (Utilities|IsValid Tile
        (:Is%20Valid
          (if (Utilities|Enum|Equal(Enum) _color "NewEnumerator8")
            (for _array_element_5 _board
              _)))))))

(fn CheckTile
  (for _array_element (Variables|Default|GetBoard)
    (Utilities|IsValid _array_element
      (:Is%20Valid
        (Utilities|FlowControl|DoOnce false
          (:Completed
            (Development|PrintString "valid"))))
      (:Is%20Not%20Valid
        (Development|PrintString "no block")
        (if (Utilities|IsValid (Utilities|Array|Get(acopy) (Variables|Default|GetBoard) (Variables|Default|GetCurrent%20Tile)))
          (Development|PrintString "invalid")
          (Components|StaticMesh|SetStaticMesh (Variables|/Game/_blueprints/BP_Tile.BP_Tile_C|GetStaticMesh _array_element) 0))))))

(fn DropTile
  (params (TileToDrop :type BP%20Tile%20Object%20Reference) (Vector :type Vector))
  (Transformation|SetWorldLocation (Variables|/Game/_blueprints/BP_Tile.BP_Tile_C|GetStaticMesh TileToDrop) Vector true false))