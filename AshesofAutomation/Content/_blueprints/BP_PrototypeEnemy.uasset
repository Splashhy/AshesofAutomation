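; Prototype enemy actor with a widget health bar, a delayed attack on the player and death handling that can open the victory level.
; BeginPlay caches WB_HealthBar and calls TakeDamage, which refreshes the bar but never stores reduced health.
; AttackPlayer, not started by BeginPlay, checks the GameMode barrier to either hit the player and recurse or lower a separate EnemyHealth.
; Much of the health-bar and timer logic is disconnected.
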(event Custom|Attack%20Player
  (params (damage :type Float%20%28double-precision%29))
  (bind _asgm_gamemode (Utilities|Casting|CastToGM_Gamemode (Game|GetGameMode)))
  (if (Variables|/Game/_blueprints/GM_Gamemode.GM_Gamemode_C|GetBarrierOn _asgm_gamemode)
    (Utilities|FlowControl|Delay 5.0)
    (CallFunction|AttacksPlayer damage)
    (Default|TakeDamage _asgm_gamemode)
    (CallFunction|AttackPlayer damage)
    (if (<= (Variables|Default|GetEnemyHealth) 0)
      (bind _output_get (Variables|Default|SetEnemies%20Killed (+ (Variables|Default|GetEnemies%20Killed) 1)))
      (if (>= _output_get 1)
        (Game|OpenLevel(byObjectReference) "/Game/_levels/Levels/VictoryScreen.VictoryScreen")
        (else
          (Actor|DestroyActor)
          (Audio|PlaySoundatLocation "/Game/Audio/dragon-studio-explosion-effect-494317.dragon-studio-explosion-effect-494317" "0, 0, 0" "0, 0, 0" 1.0 1.0 0.0 0 0 0 0))))
    (else
      (Utilities|FlowControl|Delay 5.0)
      (Variables|Default|SetEnemyHealth (Math|Float|Truncate (- (Variables|Default|GetEnemyHealth) damage))))))

(event Custom|Update%20HealthBar
  (bind _aswb_health_bar (Utilities|Casting|CastToWB_HealthBar (UserInterface|GetWidget (Variables|Default|GetHealthBar%20Widget)))))

(event EventBeginPlay
  (Variables|Default|SetEnemy%20Health%20Var (Variables|Default|GetEnemy%20Max%20Health%20Var))
  (bind _aswb_health_bar (Utilities|Casting|CastToWB_HealthBar (UserInterface|GetUserWidgetObject (Variables|Default|GetHealthBar%20Widget))))
  (Variables|Default|SetHealthBarRef _aswb_health_bar)
  (CallFunction|TakeDamage 1.0))

(event EventTick
  (params (DeltaSeconds :type Float%20%28single-precision%29)))

(fn ConstructionScript)

(fn AttacksPlayer
  (params (damage :type Float%20%28double-precision%29))
  (Utilities|DamagePlayer damage)
  (Development|PrintString "Attakced Player" true true "(R=0.312500,G=0.001250,B=0.000042,A=1.000000)"))

(fn SetEnemyHealth
  (Utilities|FlowControl|Sequence
    (:then_0
      (bind _asgm_gamemode (Utilities|Casting|CastToGM_Gamemode (Game|GetGameMode)))
      (CallFunction|AttackPlayer 0.0)
      (bind _output_get (Variables|Default|SetEnemy%20Health (Variables|/Game/_blueprints/GM_Gamemode.GM_Gamemode_C|GetEnemyHealth _asgm_gamemode)))
      (return (/ _output_get (Variables|/Game/_blueprints/GM_Gamemode.GM_Gamemode_C|GetMax%20Enemy%20Health _asgm_gamemode)) (Variables|/Game/UI/Enemy/WB_HealthBar.WB_HealthBar_C|GetBar (stale _aswb_health_bar))))
    (:then_1
      (bind _aswb_health_bar (Utilities|Casting|CastToWB_HealthBar (UserInterface|GetWidget (Variables|Default|GetHealthBar%20Widget)))))))

(fn TakeDamage
  (params (DamageAmount :type Float%20%28double-precision%29))
  (CallFunction|UpdateEnemyHealthBar)
  (if (<= (Math|Float|Clamp(Float) (- (Variables|Default|GetEnemy%20Health%20Var) DamageAmount) 0.0 (Variables|Default|GetEnemy%20Max%20Health%20Var)) 0.0)
    (Actor|DestroyActor)))

(fn UpdateEnemyHealthBar
  (bind _healthbarref (Variables|Default|GetHealthBarRef))
  (bind _bar (Variables|/Game/UI/Enemy/WB_HealthBar.WB_HealthBar_C|GetBar _healthbarref))
  (Utilities|IsValid _healthbarref
    (:Is%20Valid
      (Development|PrintString "Hello")
      (bind _output_get (Variables|/Game/UI/Enemy/WB_HealthBar.WB_HealthBar_C|SetEnemy%20Health%20 _healthbarref (Variables|Default|GetEnemy%20Health%20Var)))
      (bind _output_get_2 (Variables|/Game/UI/Enemy/WB_HealthBar.WB_HealthBar_C|SetEnemy%20Max%20Health _healthbarref (Variables|Default|GetEnemy%20Max%20Health%20Var)))
      (if (> _output_get_2 0.0)
        (Progress|SetPercent _bar (/ _output_get _output_get_2))
        (else
          (Progress|SetPercent _bar 0.0))))
    (:Is%20Not%20Valid
      (Development|PrintString "No"))))