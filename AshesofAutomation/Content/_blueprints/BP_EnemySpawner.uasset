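; Enemy spawner actor that creates enemies at its own transform from a queue of enemy classes.
; AddEnemyToQueue appends a class and immediately spawns the front entry if no prototype enemy overlaps its sphere.
; A looping timer started at BeginPlay triggers further spawn attempts, without that overlap check.
; The event graph also holds a hardcoded BP_PrototypeEnemy spawn event and an unconnected delayed debug spawn.
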(event Custom|SpawnEnemy
  (bind _returnvalue (Transformation|GetActorTransform))
  (Game|SpawnActorfromClass "/Game/_blueprints/BP_PrototypeEnemy.BP_PrototypeEnemy_C" (Math|Transform|MakeTransform (.location _returnvalue) (.rotation _returnvalue) "1.000000,1.000000,1.000000") "AdjustIfPossibleButAlwaysSpawn" "MultiplyWithRoot" 0 0))

(event Custom|TryTo%20Spawn
  (CallFunction|SpawnEnemy))

(event EventBeginPlay
  (Utilities|Time|SetTimerbyEvent (delegate Custom|TryTo%20Spawn) 2.0 true))

(fn ConstructionScript)

(fn SpawnEnemy
  (if (Utilities|Array|IsValidIndex (Variables|Default|GetEnemyQueue))
    (Game|SpawnActorfromClass (Utilities|Array|Get(acopy) (Variables|Default|GetEnemyQueue)) (Transformation|GetActorTransform) "Undefined" "MultiplyWithRoot" 0 0)
    (Utilities|Array|RemoveIndex (Variables|Default|GetEnemyQueue))
    (return true)
    (else
      (return false))))

(fn AddEnemytoQueue
  (params (Enemy%20Class :type BP%20Prototype%20Enemy%20Class%20Reference%20%28by%20ref%29))
  (Utilities|Array|Add (Variables|Default|GetEnemyQueue) Enemy%20Class)
  (if (not (Utilities|Array|IsValidIndex (Collision|GetOverlappingActors (Variables|Default|GetSphere) "/Game/_blueprints/BP_PrototypeEnemy.BP_PrototypeEnemy_C" :!class /Script/Engine.PrimitiveComponent)))
    (CallFunction|SpawnEnemy)))